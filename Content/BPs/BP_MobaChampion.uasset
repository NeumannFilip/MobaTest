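; BP_MobaChampion is a MOBA champion pawn that supports click-to-move and WASD movement.
; MoveToMarker traces from the mouse cursor on Visibility and sends the hit location to AIMoveTo.
; A test variant requires BP_CharacterController and sets IsMovingToClick, cleared only on move success, to block camera-yaw-relative Enhanced Input movement.
; The MovementWASD graph holds an unwired copy of the movement logic.
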(event `MoveToMarker`
  (bind (_worldlocation _worlddirection) (`PlayerController.DeprojectMousePositionToWorld` (`GameplayStatics.GetPlayerController` 0)))
  ;[1 1 1] Click To Move Logic
  (bind _outhit (`KismetSystemLibrary.LineTraceSingle` _worldlocation (+ _worldlocation (* _worlddirection 10000.0)) "TraceTypeQuery1"))
  (bind _output_get (set `self.Location` (`.Location` (`GameplayStatics.BreakHitResult` _outhit))))
  (`|AIMoveTo` self _output_get null))

(event `MoveToMarkerTest`
  ;[1 1 1] Test to make it work with WSAD Movement
  (bind _asbp_character_controller (cast `/Game/BPs/BP_CharacterController` (`GameplayStatics.GetPlayerController` 0)))
  (bind (_worldlocation _worlddirection) (`PlayerController.DeprojectMousePositionToWorld` _asbp_character_controller))
  (bind _outhit (`KismetSystemLibrary.LineTraceSingle` _worldlocation (+ _worldlocation (* _worlddirection 10000.0)) "TraceTypeQuery1"))
  (bind _output_get (set `self.Location` (`.Location` (`GameplayStatics.BreakHitResult` _outhit))))
  (`|AIMoveTo` self _output_get null
    (:`then`
      (set `self.IsMovingToClick` true))
    (:`OnSuccess`
      (set `self.IsMovingToClick` false))))

(event `EnhancedInput|/Game/Input/IA_MoveForward`
  (params (ActionValue :type "Vector2D Structure") (ElapsedSeconds :type "Float (double-precision)") (TriggeredSeconds :type "Float (double-precision)") (InputAction :type "InputAction Object Reference" :default "/Game/Input/IA_MoveForward.IA_MoveForward"))
  (bind (_returnvalue_roll _returnvalue_pitch _returnvalue_yaw) (`KismetMathLibrary.BreakRotator` (`self.GetControlRotation`)))
  (bind _returnvalue (`KismetMathLibrary.MakeRotator` 0.0 0.0 _returnvalue_yaw))
  ;[1 1 1] Test to make it work with WSAD Movement
  (:`Triggered`
    (if (not (`self.IsMovingToClick`))
      (`|ExecutionSequence`
        (:`then_0`
          (`self.AddMovementInput` (`KismetMathLibrary.GetRightVector` _returnvalue) ActionValue_Y))
        (:`then_1`
          (`self.AddMovementInput` (`KismetMathLibrary.GetForwardVector` _returnvalue) ActionValue_X))))))

(event `EnhancedInput|/Game/Input/IA_MoveForward`
  (params (ActionValue :type "Vector2D Structure") (ElapsedSeconds :type "Float (double-precision)") (TriggeredSeconds :type "Float (double-precision)") (InputAction :type "InputAction Object Reference" :default "/Game/Input/IA_MoveForward.IA_MoveForward")))

(fn `UserConstructionScript`)