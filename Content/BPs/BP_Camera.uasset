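; Camera actor that becomes the player's view target at BeginPlay and supports planar panning and zooming.
; Zoom input adjusts a clamped target factor and restarts a timeline that eases the spring arm length toward it.
; MoveCamera offsets the actor in world XY by frame-time-scaled speed.
; The timeline also sets that speed, derived solely from the initial speed rather than the zoom factor.
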(event `self.ReceiveBeginPlay`
  (`PlayerController.SetViewTargetWithBlend` (`GameplayStatics.GetPlayerController` 0) self 0.0 "VTBlend_Linear" 0.0 false)
  (set `self.DesiredZoomFactor` 0.5)
  (bind (_direction _zoomcameratrack) (`Timeline|ZoomCameraTimeline` :!via `PlayFromStart` :!label _label)
    (:`Update`
      (bind _returnvalue (`KismetMathLibrary.Lerp` (`self.ZoomFactor`) (`self.DesiredZoomFactor`) _zoomcameratrack))
      (set `self.ZoomFactor` _returnvalue)
      (set `SpringArmComponent.TargetArmLength` (`KismetMathLibrary.Lerp` 200.0 1500.0 _returnvalue) (`self.SpringArm`))
      (set `self.CameraSpeed` (* (`KismetMathLibrary.FClamp` (`self.InitCameraSpeed`) 0.35 0.8) (`self.InitCameraSpeed`))))))

(event `Zoom`
  (params (MouseWheelAxis :type "Float (double-precision)"))
  (set `self.DesiredZoomFactor` (`KismetMathLibrary.FClamp` (+ (`self.DesiredZoomFactor`) (/ MouseWheelAxis (`self.ZoomSpeed`)))))
  (goto _label :!via `PlayFromStart`))

(fn `MoveCamera`
  (params (XDir :type "Float (double-precision)") (YDir :type "Float (double-precision)"))
  ;[1 1 1] Camera Movement
  (`self.K2_AddActorWorldOffset` (`KismetMathLibrary.MakeVector` (* (* XDir (`self.CameraSpeed`)) (`GameplayStatics.GetWorldDeltaSeconds`)) (* (* YDir (`self.CameraSpeed`)) (`GameplayStatics.GetWorldDeltaSeconds`)))))

(fn `UserConstructionScript`)