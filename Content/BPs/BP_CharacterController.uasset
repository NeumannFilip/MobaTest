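; Character controller for a MOBA-style game that forwards click-to-move input to the controlled champion.
; The IA_ClickToMove action casts the CharacterMOba reference to BP_MobaChampion and calls its MoveToMarkerTest, leaving movement logic to the champion.
; A disconnected chain that line-traces under the mouse cursor and sends the hit location to AIMoveTo never runs.
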(event `EnhancedInput|/Game/Input/IA_ClickToMove`
  (params (ActionValue :type Boolean) (ElapsedSeconds :type "Float (double-precision)") (TriggeredSeconds :type "Float (double-precision)") (InputAction :type "InputAction Object Reference" :default "/Game/Input/IA_ClickToMove.IA_ClickToMove"))
  (bind _charactermoba (`self.CharacterMOba`))
  ;[1 1 1] test
  (:`Triggered`
    (cast `/Game/BPs/BP_MobaChampion` _charactermoba)
    (`/Game/BPs/BP_MobaChampion.MoveToMarkerTest` _charactermoba)))

(event `Key|LeftMouseButton`
  (params (Key :type "Key Structure"))
  ;[1 1 1] test
)

(fn `UserConstructionScript`)